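; Test player controller for a time-attack racing game that runs the race start countdown.
; The first left mouse press, gated by a DoOnce, broadcasts that the player has started the game and steps ReadyText from "3" to "Go" using timed delays.
; It then broadcasts that the player is ready, sets the race-started flag and starts the race and lap timers.
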(event `InputAction|LeftMouse`
  (params (Key :type "Key Structure" :default "AnyKey"))
  (:`Pressed`
    (`/Engine/EditorBlueprintResources/StandardMacros.DoOnce` false
      (:`Completed`
        (`self.PlayerHasStartTheGame`)
        (set `self.ReadyText` "3")
        (`KismetSystemLibrary.Delay` 2.5)
        (set `self.ReadyText` "2")
        (`KismetSystemLibrary.Delay` 1.0)
        (set `self.ReadyText` "1")
        (`KismetSystemLibrary.Delay` 1.0)
        (set `self.ReadyText` "Go")
        (`KismetSystemLibrary.Delay` 1.0)
        (`self.PlayerIsReadyToStart`)
        (set `self.RaceStart` true)
        (`self.StartRaceTime`)
        (`self.StartLapTime`)))))

(fn `UserConstructionScript`)