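; GameStateManager is an actor that wires checkpoint tracking into the time attack racer's game state and respawn system.
; On BeginPlay it hands its TrackerManager reference to MyGameStateBP, calls InitText there, and binds to the tracker's checkpoint-cleared event.
; Each cleared checkpoint sets the first player controller's RespawnLocation to that checkpoint's transform.
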(event `self.ReceiveBeginPlay`
  (bind _asmy_game_state_bp (cast `/Game/TimeAttackRacer/Blueprints/MyGameStateBP` (`GameplayStatics.GetGameState`)))
  (set `MyGameStateBase.TrackerManager` (`self.TrackerManager`) _asmy_game_state_bp)
  (`MyGameStateBase.InitText` _asmy_game_state_bp)
  (add `Tracker.OnCheckPointClearedF` (`self.TrackerManager`) (delegate `OnCheckPointCleared`)))

(event `OnCheckPointCleared`
  (params (CheckPoint :type "Checkpoint Object Reference"))
  (bind _asmy_player_controller (cast `MyPlayerController` (`GameplayStatics.GetPlayerController` 0)))
  (set `MyPlayerController.RespawnLocation` (`self.GetTransform` CheckPoint) _asmy_player_controller))

(fn `UserConstructionScript`)