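; Spline-based race track generator that builds road and guard rail meshes in the Construction Script.
; It resizes a per-point road data array to match the spline point count, filling new entries from defaults.
; Each segment gets spline meshes with per-point bank, width and thickness, optional left/right rails and toggleable collision, wrapping around for looping tracks.
; An optional debug pass labels each spline point with its index.
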(event `self.ReceiveBeginPlay`)

(fn `BuildTrackElement`
  (params (LoopIndex :type Integer) (TrackElementMesh :type "StaticMesh Object Reference"))
  (locals (Local_CurrentLoopIndex :type Integer) (Local_NextLoopIndex :type Integer :default 0) (Local_TrackElementMesh :type "StaticMesh Object Reference") (Local_StartLocation :type "Vector Structure") (Local_StartTangent :type "Vector Structure") (Local_EndLocation :type "Vector Structure") (Local_EndTangent :type "Vector Structure") (Local_CurrentSplineMesh :type "SplineMeshComponent Object Reference") (Local_StartRoll :type "Float (double-precision)") (Local_StartScale :type "Vector2D Structure") (Local_EndRoll :type "Float (double-precision)") (Local_EndScale :type "Vector2D Structure"))
  (bind _local_currentsplinemesh (`local.Local_CurrentSplineMesh`))
  (bind (_item_leftguardrail _item_rightguardrail _item_trackbank _item_trackwidth _item_trackthickness) (break `/Game/TimeAttackRacer/Blueprints/DataTrack/RoadData` (`KismetArrayLibrary.Array_Get` (`self.Road Data Array`) (`local.Local_NextLoopIndex`))))
  (bind (_item_leftguardrail_2 _item_rightguardrail_2 _item_trackbank_2 _item_trackwidth_2 _item_trackthickness_2) (break `/Game/TimeAttackRacer/Blueprints/DataTrack/RoadData` (`KismetArrayLibrary.Array_Get` (`self.Road Data Array`) (`local.Local_CurrentLoopIndex`))))
  (bind (_location _tangent) (`SplineComponent.GetLocationAndTangentAtSplinePoint` (`self.Spline`) (`local.Local_NextLoopIndex`) "Local"))
  (bind (_location_2 _tangent_2) (`SplineComponent.GetLocationAndTangentAtSplinePoint` (`self.Spline`) (`local.Local_CurrentLoopIndex`) "Local"))
  (set `local.Local_CurrentLoopIndex` LoopIndex)
  (set `local.Local_NextLoopIndex` (mod (+ LoopIndex 1) (`self.Number Of Spline Point`)))
  (set `local.Local_TrackElementMesh` TrackElementMesh)
  (`|ExecutionSequence`
    (:`then_0`
      (set `local.Local_StartLocation` _location_2)
      (set `local.Local_StartTangent` _tangent_2)
      (set `local.Local_EndLocation` _location)
      (set `local.Local_EndTangent` _tangent)
      (set `local.Local_StartRoll` _item_trackbank_2)
      (set `local.Local_StartScale` (`KismetMathLibrary.MakeVector2D` _item_trackwidth_2 _item_trackthickness_2))
      (set `local.Local_EndRoll` _item_trackbank)
      (set `local.Local_EndScale` (`KismetMathLibrary.MakeVector2D` _item_trackwidth _item_trackthickness)))
    (:`then_1`
      (bind _returnvalue (`AddComponent|NODE_AddSplineMeshComponent-0`))
      (set `local.Local_CurrentSplineMesh` _returnvalue)
      (`StaticMeshComponent.SetStaticMesh` (`local.Local_CurrentSplineMesh`) (`local.Local_TrackElementMesh`))
      (`SplineMeshComponent.SetStartAndEnd` (`local.Local_CurrentSplineMesh`) (`local.Local_StartLocation`) (`local.Local_StartTangent`) (`local.Local_EndLocation`) (`local.Local_EndTangent`) true)
      (`SplineMeshComponent.SetStartRoll` _local_currentsplinemesh (`local.Local_StartRoll`) true)
      (`SplineMeshComponent.SetEndRoll` _local_currentsplinemesh (`local.Local_EndRoll`) true)
      (`SplineMeshComponent.SetStartScale` (`local.Local_CurrentSplineMesh`) (`local.Local_StartScale`) true)
      (`SplineMeshComponent.SetEndScale` (`local.Local_CurrentSplineMesh`) (`local.Local_EndScale`) true)
      (`PrimitiveComponent.SetCollisionEnabled` (`local.Local_CurrentSplineMesh`) (select `bool` (`self.Collissions`) :`false` "NoCollision" :`true` "QueryAndPhysics" :!type "ECollisionEnabled Enum")))))

(fn `UserConstructionScript`
  (bind _road_data_array (`self.Road Data Array`))
  (`|ExecutionSequence`
    (:`then_0`
      (set `self.Number Of Spline Point` (`SplineComponent.GetNumberOfSplinePoints` (`self.Spline`))))
    (:`then_1`
      (`/Engine/EditorBlueprintResources/StandardMacros.CompareInt` (`KismetArrayLibrary.Array_Length` (`self.Road Data Array`)) (`self.Number Of Spline Point`) :!label _label
        (:`>`
          (`KismetArrayLibrary.Array_Remove` _road_data_array (`KismetArrayLibrary.Array_LastIndex` _road_data_array))
          (goto _label))
        (:`<`
          (`KismetArrayLibrary.Array_Add` (`self.Road Data Array`) (`self.RoadMeshDefaults`))
          (goto _label))))
    (:`then_2`
      (for _index (range (+ (- (`self.Number Of Spline Point`) (`KismetMathLibrary.SelectInt` 1 2 (`self.LoopingTrack`))) 1))
        (set `self.CurrentLoopIndex` _index)
        (bind (_item_leftguardrail _item_rightguardrail) (break `/Game/TimeAttackRacer/Blueprints/DataTrack/RoadData` (`KismetArrayLibrary.Array_Get` (`self.Road Data Array`) _index)))
        (set `self.DrawleftGuardRail` _item_leftguardrail)
        (set `self.DrawRightGuardRail` _item_rightguardrail)
        (`|ExecutionSequence`
          (:`then_0`
            (`self.BuildTrackElement` (`self.CurrentLoopIndex`) (`self.RoadMesh`)))
          (:`then_1`
            (if (`self.DrawleftGuardRail`)
              (`self.BuildTrackElement` (`self.CurrentLoopIndex`) (`self.LeftGuardRailMesh`))))
          (:`then_2`
            (if (`self.DrawRightGuardRail`)
              (`self.BuildTrackElement` (`self.CurrentLoopIndex`) (`self.RightGuardRailMesh`)))))))
    (:`then_3`
      (if (`self.DrawTrackPointNumbers`)
        (for _index_2 (range (`self.Number Of Spline Point`))
          (set `self.CurrentTrackPoint` (`KismetStringLibrary.Conv_IntToString` _index_2))
          (bind (_location _tangent) (`SplineComponent.GetLocationAndTangentAtSplinePoint` (`self.Spline`) _index_2 "Local"))
          (bind _returnvalue (`AddComponent|NODE_AddTextRenderComponent-0` :`RelativeTransform` (`KismetMathLibrary.MakeTransform` (`KismetMathLibrary.MakeVector` (.x _location) (.y _location) (+ (.z _location) 50.0)) (`KismetMathLibrary.Conv_VectorToRotator` (* _tangent -1.0)))))
          (`TextRenderComponent.K2_SetText` _returnvalue (`KismetTextLibrary.Conv_StringToText` (`self.CurrentTrackPoint`))))))))