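; Game mode for the time-attack racer that holds the player's car until the race begins.
; On BeginPlay it caches the player controller, pawn and game state, disables pawn input and binds to the controller's player-has-started event.
; That event runs a one-second-step countdown text, then broadcasts StartTheGame, re-enables input and starts the game state's race and lap timers.
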(event `self.ReceiveBeginPlay`
  ;[1 1 1] Get Playercontroller referece, pwn reference and bind to event
  (bind _asmy_player_controller (cast `MyPlayerController` (`GameplayStatics.GetPlayerController` 0)))
  (bind _output_get (set `self.PlayerController` _asmy_player_controller))
  (add `MyPlayerController.PlayerHasStartedTheGame` _output_get (delegate `PlayerHasStartedTheGame`))
  (bind _astime_attack_racer_pawn (cast `TimeAttackRacerPawn` (`Controller.K2_GetPawn` _output_get)))
  (bind _output_get_2 (set `self.PlayerPwn` _astime_attack_racer_pawn))
  (`self.DisableInput` _output_get_2 null)
  (bind _asmy_game_state_base (cast `MyGameStateBase` (`GameplayStatics.GetGameState`)))
  (set `self.MyGameState` _asmy_game_state_base))

(event `PlayerHasStartedTheGame`
  ;[1 1 1] Player Request to Start the Game EVENT
  (set `self.ReadyText` "3")
  (`KismetSystemLibrary.Delay` 1.0)
  (set `self.ReadyText` "2")
  (`KismetSystemLibrary.Delay` 1.0)
  (set `self.ReadyText` "1")
  (`KismetSystemLibrary.Delay` 1.0)
  (set `self.ReadyText` "GO!")
  (`KismetSystemLibrary.Delay` 1.0)
  (`self.StartTheGameEvent`))

(event `StartTheGameEvent`
  (bind _mygamestate (`self.MyGameState`))
  (`self.StartTheGame`)
  (`self.EnableInput` (`self.PlayerPwn`) null)
  (`MyGameStateBase.StartRaceTime` _mygamestate)
  (`MyGameStateBase.StartLapTime` _mygamestate))

(fn `UserConstructionScript`)